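; BP_Layered is an actor that shows a stack of floor actors layer by layer, lifting away those above a selected index.
; BeginPlay records each floor's original location and selects the top floor; SelectedCurrentIndex sets the active index after validating it.
; Each Tick eases floors above the selection up by Height and the rest back home, snapping near the target and hiding raised floors on arrival.
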(event Custom|SelectedCurrentIndex
  (params (CurrentSelectedIndex :type Integer))
  (if (Utilities|Array|IsValidIndex (Variables|Default|GetFloors) CurrentSelectedIndex)
    (Variables|Default|SetCurrentSelectedIndex CurrentSelectedIndex)))

(event EventBeginPlay
  (bind _floors (Variables|Default|GetFloors))
  (Utilities|Array|Clear (Variables|Default|GetDefaultLocs))
  (for _array_element _floors
    (Utilities|Array|Add (Variables|Default|GetDefaultLocs) (Transformation|GetActorLocation _array_element)))
  (CallFunction|SelectedCurrentIndex (Utilities|Array|LastIndex _floors)))

(event Collision|EventActorBeginOverlap
  (params (OtherActor :type Actor%20Object%20Reference)))

(event EventTick
  (params (DeltaSeconds :type Float%20%28single-precision%29))
  (for (_array_element _array_index) (Variables|Default|GetFloors)
    (Utilities|IsValid _array_element
      (:Is%20Valid
        (Transformation|SetActorLocation _array_element (select (Utilities|Operators|EqualEqual (Transformation|GetActorLocation _array_element) (select (> _array_index (Variables|Default|GetCurrentSelectedIndex)) (+ (Utilities|Array|Get(acopy) (Variables|Default|GetDefaultLocs) _array_index) (* "0.000000,0.000000,1.000000" (Variables|Default|GetHeight))) (Utilities|Array|Get(acopy) (Variables|Default|GetDefaultLocs) _array_index)) 35.0) (select (> _array_index (Variables|Default|GetCurrentSelectedIndex)) (+ (Utilities|Array|Get(acopy) (Variables|Default|GetDefaultLocs) _array_index) (* "0.000000,0.000000,1.000000" (Variables|Default|GetHeight))) (Utilities|Array|Get(acopy) (Variables|Default|GetDefaultLocs) _array_index)) (Math|Interpolation|VInterpTo (Transformation|GetActorLocation _array_element) (select (> _array_index (Variables|Default|GetCurrentSelectedIndex)) (+ (Utilities|Array|Get(acopy) (Variables|Default|GetDefaultLocs) _array_index) (* "0.000000,0.000000,1.000000" (Variables|Default|GetHeight))) (Utilities|Array|Get(acopy) (Variables|Default|GetDefaultLocs) _array_index)) DeltaSeconds 5.0)) false false)
        (Rendering|SetActorHiddenInGame _array_element (and (Utilities|Operators|EqualEqual (Transformation|GetActorLocation _array_element) (select (> _array_index (Variables|Default|GetCurrentSelectedIndex)) (+ (Utilities|Array|Get(acopy) (Variables|Default|GetDefaultLocs) _array_index) (* "0.000000,0.000000,1.000000" (Variables|Default|GetHeight))) (Utilities|Array|Get(acopy) (Variables|Default|GetDefaultLocs) _array_index)) 35.0) (> _array_index (Variables|Default|GetCurrentSelectedIndex))))))))

(fn ConstructionScript)