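; BP_RoomBase is a base room Blueprint with helpers for reading and setting material opacity on its static mesh.
; The construction script creates a dynamic instance for each material slot and stores them in MaterialsIns.
; GetOpactityValue reads "OpacityValue" from the first instance, while SetOpactityValue writes to every instance using parameter name "None" rather than "OpacityValue".
; Nothing in the event graph runs or calls these helpers.
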(event EventBeginPlay)

(event Collision|EventActorBeginOverlap
  (params (OtherActor :type Actor%20Object%20Reference)))

(event EventTick
  (params (DeltaSeconds :type Float%20%28single-precision%29)))

(fn ConstructionScript
  (for (_array_element _array_index) (Rendering|Material|GetMaterials (Variables|Default|GetStaticMesh))
    (bind _returnvalue (Rendering|Material|CreateDynamicMaterialInstance (Variables|Default|GetStaticMesh) _array_index _array_element "OpacityValue" :!class /Script/Engine.PrimitiveComponent))
    (Utilities|Array|Add (Variables|Default|GetMaterialsIns) _returnvalue)))

(fn GetOpactityValue
  (bind _returnvalue (Rendering|Material|GetScalarParameterValue (Utilities|Array|Get(acopy) (Variables|Default|GetMaterialsIns)) "OpacityValue" :!class /Script/Engine.MaterialInstanceDynamic))
  (return _returnvalue))

(fn SetOpactityValue
  (params (Value :type Float%20%28single-precision%29))
  (for _array_element (Variables|Default|GetMaterialsIns)
    (Rendering|Material|SetScalarParameterValue _array_element "None" Value :!class /Script/Engine.MaterialInstanceDynamic)))